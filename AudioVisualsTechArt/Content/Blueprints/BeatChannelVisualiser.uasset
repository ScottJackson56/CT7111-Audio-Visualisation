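; BeatChannelVisualiser is an actor that shows audio beats by changing the height of a left and right cube.
; Each Tick it reads BeatPeakSwitch from the first AudioHost and sets both cubes' Z scale to BeatIntensityOn or BeatIntensityOff.
; A peak also sets Pause, which routes later ticks through a Delay of Buffer length; this graph never clears Pause.
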(event Collision|EventActorBeginOverlap
  (params (OtherActor :type Actor%20Object%20Reference)))

(event EventTick
  (params (DeltaSeconds :type Float%20%28single-precision%29))
  (bind _beatintensityon (Variables|Default|GetBeatIntensityOn))
  (bind _beatintensityoff (Variables|Default|GetBeatIntensityOff))
  (bind _outactors (Actor|GetAllActorsOfClass "/Game/Blueprints/AudioHost.AudioHost_C"))
  (if (Variables|Default|GetPause)
    (Utilities|FlowControl|Delay (Variables|Default|GetBuffer)))
  (if (Variables|/Game/Blueprints/AudioHost.AudioHost_C|GetBeatPeakSwitch (Utilities|Array|Get(acopy) _outactors))
    (Transformation|SetRelativeScale3D (Variables|Default|GetLeftCube) (Math|Vector|MakeVector 1.0 1.0 _beatintensityon))
    (Transformation|SetRelativeScale3D (Variables|Default|GetRightCube) (Math|Vector|MakeVector 1.0 1.0 _beatintensityon))
    (Variables|Default|SetPause true)
    (else
      (Transformation|SetRelativeScale3D (Variables|Default|GetLeftCube) (Math|Vector|MakeVector 1.0 1.0 _beatintensityoff))
      (Transformation|SetRelativeScale3D (Variables|Default|GetRightCube) (Math|Vector|MakeVector 1.0 1.0 _beatintensityoff)))))

(fn ConstructionScript)