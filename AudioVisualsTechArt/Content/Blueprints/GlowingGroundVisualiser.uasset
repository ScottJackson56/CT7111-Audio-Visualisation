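; GlowingGroundVisualiser is an audio-reactive actor whose static mesh brightness follows sound loudness.
; BeginPlay creates a dynamic material instance on the mesh and applies the initial Brightness.
; Each Tick looks up the first AudioHost actor, averages its normalised left and right channel loudness, and writes the result to the material's Brightness parameter.
; The BrightnessOnBeat function is an empty stub.
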(event EventBeginPlay
  (bind _staticmesh (Variables|Default|GetStaticMesh))
  (Rendering|Material|CreateDynamicMaterialInstance _staticmesh 0 (Rendering|Material|GetMaterial _staticmesh 0) "None" :!class /Script/Engine.PrimitiveComponent)
  (Rendering|Material|SetScalarParameterValueonMaterials (Variables|Default|GetStaticMesh) "Brightness" (stale EventTick _output_get)))

(event EventTick
  (params (DeltaSeconds :type Float%20%28single-precision%29))
  (bind _outactors (Actor|GetAllActorsOfClass "/Game/Blueprints/AudioHost.AudioHost_C"))
  (bind _output_get (Variables|Default|SetBrightness (/ (+ (Variables|/Game/Blueprints/AudioHost.AudioHost_C|GetNormalised%20Right%20Channel%20Loudness (Utilities|Array|Get(acopy) _outactors)) (Variables|/Game/Blueprints/AudioHost.AudioHost_C|GetNormalised%20Left%20Channel%20Loudness (Utilities|Array|Get(acopy) _outactors))) 2.0)))
  (Rendering|Material|SetScalarParameterValueonMaterials (Variables|Default|GetStaticMesh) "Brightness" _output_get))

(fn ConstructionScript)

(fn BrightnessonBeat)