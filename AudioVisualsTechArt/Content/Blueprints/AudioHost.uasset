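; AudioHost plays a sound and exposes time-synced audio analysis values for audio-reactive visuals.
; The construction script takes the sound and duration from its loudness analyser asset.
; Each playback-percent update samples offline loudness per channel and Constant-Q band strengths, averages loudness and thresholds it into a beat switch.
; It also drives the HueShift material parameter collection value from a curve over playback progress.
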(event Custom|PlaybackPercentEvent
  (params (PlayingSoundWave :type Sound%20Wave%20Object%20Reference) (PlaybackPercent :type Float%20%28single-precision%29))
  (bind _duration (Variables|Default|GetDuration))
  (bind _returnvalue (* PlaybackPercent _duration))
  (Variables|Default|SetCurrentPlayback _returnvalue)
  (Utilities|FlowControl|Sequence
    (:then_0
      ;[1 1 1] Normalised Left and Right Channel Volumes
      (bind _output_get (Variables|Default|SetNormalised%20Left%20Channel%20Loudness (Class|LoudnessNRT|GetNormalizedChannelLoudnessatTime (Variables|Default|GetLoudnessAnalyser) _returnvalue)))
      (bind _output_get_2 (Variables|Default|SetNormalised%20Right%20Channel%20Loudness (Class|LoudnessNRT|GetNormalizedChannelLoudnessatTime (Variables|Default|GetLoudnessAnalyser) _returnvalue 1)))
      (Variables|Default|SetNormalisedGeneralLoudness (/ (+ _output_get _output_get_2) 2.0)))
    (:then_1
      ;[1 1 1] Constant Band Values
      (Variables|Default|SetConstantBandStrength (Class|ConstantQNRT|GetNormalizedChannelConstantQatTime (Variables|Default|GetConstantAnalyser) _returnvalue)))
    (:then_2
      ;[1 1 1] Beat Switch State
      (Utilities|FlowControl|Sequence
        (:then_0
          (Variables|Default|SetBeatPeakSwitch (>= (Variables|Default|GetNormalisedGeneralLoudness) (Variables|Default|GetNormalisedSwitchLimit))))))
    (:then_3
      (Rendering|Material|SetScalarParameterValue "/Game/Materials/NPC_HueShift.NPC_HueShift" "HueShift" (Math|Curves|GetFloatValue (Variables|Default|GetHueCurve) PlaybackPercent) :!class /Script/Engine.KismetMaterialLibrary))))

(event EventBeginPlay
  (bind _audio (Variables|Components|GetAudio))
  (EventDispatchers|BindEventtoOnAudioPlaybackPercent _audio (delegate Custom|PlaybackPercentEvent))
  (Audio|Components|Audio|Play _audio 0.0))

(fn ConstructionScript
  (bind _loudnessanalyser (Variables|Default|GetLoudnessAnalyser))
  (bind _sound (Variables|/Script/AudioAnalyzer.AudioAnalyzerNRT|GetSound _loudnessanalyser))
  (Audio|Components|Audio|SetSound (Variables|Components|GetAudio) _sound)
  (Variables|Default|SetDuration (Variables|/Script/Engine.SoundBase|GetDuration _sound)))

(fn ConstantVisScaling
  (params (CurrentPlayback :type Float%20%28double-precision%29))
  (Utilities|FlowControl|Sequence
    (:then_0
      (Variables|Default|SetAudioPosition CurrentPlayback))
    (:then_1
      (Variables|Default|SetConstantBandStrength (Class|ConstantQNRT|GetNormalizedChannelConstantQatTime (Variables|Default|GetConstantAnalyser) (Variables|Default|GetAudioPosition))))))