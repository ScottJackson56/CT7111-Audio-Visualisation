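; LRChannelVisualiser is an actor that visualises stereo audio loudness with a left and a right cube.
; Each Tick it finds the first AudioHost actor via GetAllActorsOfClass, without caching it, and reads its normalised left and right channel loudness.
; Each cube's Z scale is set to its channel's loudness multiplied by the host's GlobalIntensity.
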(event Collision|EventActorBeginOverlap
  (params (OtherActor :type Actor%20Object%20Reference)))

(event EventTick
  (params (DeltaSeconds :type Float%20%28single-precision%29))
  (bind _outactors (Actor|GetAllActorsOfClass "/Game/Blueprints/AudioHost.AudioHost_C"))
  (Variables|Default|SetNLC (Variables|/Game/Blueprints/AudioHost.AudioHost_C|GetNormalised%20Left%20Channel%20Loudness (Utilities|Array|Get(acopy) _outactors)))
  (Variables|Default|SetNRC (Variables|/Game/Blueprints/AudioHost.AudioHost_C|GetNormalised%20Right%20Channel%20Loudness (Utilities|Array|Get(acopy) _outactors)))
  (Transformation|SetRelativeScale3D (Variables|Default|GetLeftCube) (Math|Vector|MakeVector 1.0 1.0 (* (Variables|Default|GetNLC) (Variables|/Game/Blueprints/AudioHost.AudioHost_C|GetGlobalIntensity (Utilities|Array|Get(acopy) _outactors)))))
  (Transformation|SetRelativeScale3D (Variables|Default|GetRightCube) (Math|Vector|MakeVector 1.0 1.0 (* (Variables|Default|GetNRC) (Variables|/Game/Blueprints/AudioHost.AudioHost_C|GetGlobalIntensity (Utilities|Array|Get(acopy) _outactors))))))

(fn ConstructionScript)