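; ActiveSkybox is an audio-reactive skybox actor that rotates and pulses its star brightness with sound loudness.
; BeginPlay creates a dynamic material instance on its mesh and sets the initial material parameters.
; Each Tick adds a fixed pitch step unscaled by delta time and averages left and right loudness from the first AudioHost found.
; It then pushes brightness, strength and the NPC_HueShift collection's hue to the material.
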(event EventBeginPlay
  (bind _staticmesh (Variables|Default|GetStaticMesh))
  (bind _staticmesh_2 (Variables|Default|GetStaticMesh))
  (Rendering|Material|CreateDynamicMaterialInstance _staticmesh 0 (Rendering|Material|GetMaterial _staticmesh 0) "None" :!class /Script/Engine.PrimitiveComponent)
  (Rendering|Material|SetScalarParameterValueonMaterials _staticmesh_2 "Brightness" (stale EventTick _output_get))
  (Rendering|Material|SetScalarParameterValueonMaterials _staticmesh_2 "GlobalStrength" (Variables|Default|GetGlobalStrength))
  (Rendering|Material|SetScalarParameterValueonMaterials _staticmesh_2 "SceneBrightness" (Variables|Default|GetSceneBrightness))
  (Rendering|Material|SetScalarParameterValueonMaterials _staticmesh_2 "Hue Shift Percentage (S)" (stale EventTick _returnvalue)))

(event EventTick
  (params (DeltaSeconds :type Float%20%28single-precision%29))
  (bind _staticmesh (Variables|Default|GetStaticMesh))
  (Transformation|AddRelativeRotation (Variables|Default|GetDefaultSceneRoot) (Math|Rotator|MakeRotator 0.0 (Variables|Default|GetRotateSpeed) 0.0) false false)
  (bind _returnvalue (Rendering|Material|GetScalarParameterValue "/Game/Materials/NPC_HueShift.NPC_HueShift" "HueShift" :!class /Script/Engine.KismetMaterialLibrary))
  (bind _outactors (Actor|GetAllActorsOfClass "/Game/Blueprints/AudioHost.AudioHost_C"))
  (bind _output_get (Variables|Default|SetStarBrightness (/ (+ (Variables|/Game/Blueprints/AudioHost.AudioHost_C|GetNormalised%20Right%20Channel%20Loudness (Utilities|Array|Get(acopy) _outactors)) (Variables|/Game/Blueprints/AudioHost.AudioHost_C|GetNormalised%20Left%20Channel%20Loudness (Utilities|Array|Get(acopy) _outactors))) 2.0)))
  (Rendering|Material|SetScalarParameterValueonMaterials _staticmesh "Brightness" _output_get)
  (Rendering|Material|SetScalarParameterValueonMaterials _staticmesh "GlobalStrength" (Variables|Default|GetGlobalStrength))
  (Rendering|Material|SetScalarParameterValueonMaterials _staticmesh "SceneBrightness" (Variables|Default|GetSceneBrightness))
  (Rendering|Material|SetScalarParameterValueonMaterials _staticmesh "Hue Shift Percentage (S)" _returnvalue))

(fn ConstructionScript)